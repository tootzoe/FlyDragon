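; BP_TestRotation is a test actor that visualizes vector rotation math with debug coordinate axes.
; The custom Unrot event rotates a variable-driven vector, unrotates it by a fixed rotator, then draws the result and prints a message.
; Tick rotates the actor's location around X by Ang, offsets it by another actor's location, and draws axes there with scaled-down Z.
; An actor-rotation node is left unconnected.
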(event `Unrot`
  (`KismetSystemLibrary.DrawDebugCoordinateSystem` (`KismetMathLibrary.LessLess_VectorRotator` (`KismetMathLibrary.GreaterGreater_VectorRotator` (`KismetMathLibrary.MakeVector` (`self.MyX`) (`self.MyY`) (`self.MyZ`)) (`KismetMathLibrary.MakeRotator` (`self.MyR`) (`self.MyP`) (`self.MyYaw`))) (struct :`Yaw` 50.0)) (struct) 120.0 33.0 3.0)
  (`KismetSystemLibrary.PrintString` "Unrotate......." true true (struct :`G` 0.66 :`B` 1.0 :`A` 1.0) 44.0))

(event `self.ReceiveTick`
  (params (DeltaSeconds :type "Float (single-precision)"))
  (bind _returnvalue (`GameplayStatics.GetActorOfClass` null))
  (bind (_returnvalue_x _returnvalue_y _returnvalue_z) (`KismetMathLibrary.BreakVector` (+ (`KismetMathLibrary.RotateAngleAxis` (`self.K2_GetActorLocation`) (`self.Ang`) (1.0 0.0 0.0)) (`self.K2_GetActorLocation` _returnvalue))))
  (`KismetSystemLibrary.DrawDebugCoordinateSystem` (`KismetMathLibrary.MakeVector` _returnvalue_x _returnvalue_y (* _returnvalue_z 0.33)) (struct) 100.0 0.2 2.0))

(fn `UserConstructionScript`)