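; Randomized VDB cloud actor that appears with a random yaw, animates its density, then destroys itself.
; The construction script builds a dynamic material from a random DT_CloudMaterials row and sets a random DT_VdbTextures sparse volume texture on it, though the parameter name is None.
; BeginPlay applies it to the HeterogeneousVolume and plays the UpdCloud timeline, whose single CloudDensity track drives both density and temperature scales.
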(event `self.ReceiveBeginPlay`
  (`PrimitiveComponent.SetMaterial` (`self.HeterogeneousVolume`) 0 (`self.VDBMatInst`))
  (`self.ShowUp`)
  (`SceneComponent.K2_SetWorldRotation` (`self.HeterogeneousVolume`) (`KismetMathLibrary.MakeRotator` 0.0 0.0 (`KismetMathLibrary.RandomFloatInRange` 0.0 360.0)) false false))

(event `ShowUp`
  (bind _vdbmatinst (`self.VDBMatInst`))
  (bind (_direction _clouddensity) (`Timeline|UpdCloud`)
    (:`Update`
      (`MaterialInstanceDynamic.SetScalarParameterValue` _vdbmatinst "Temperature Scale" _clouddensity)
      (`MaterialInstanceDynamic.SetScalarParameterValue` _vdbmatinst "Density Scale" _clouddensity))
    (:`Finished`
      (`self.K2_DestroyActor`))))

(fn `UserConstructionScript`
  (bind _outrownames (`DataTableFunctionLibrary.GetDataTableRowNames` "/Game/Materials/VDBClouds/DT_CloudMaterials.DT_CloudMaterials"))
  (bind _returnvalue (`|GetDataTableRow` "/Game/Materials/VDBClouds/DT_CloudMaterials.DT_CloudMaterials" (`KismetArrayLibrary.Array_Random` _outrownames))
    (:`then`
      (bind _returnvalue_2 (`KismetMaterialLibrary.CreateDynamicMaterialInstance` (break `/Game/Materials/VDBClouds/ST_CloudMat` _returnvalue)))
      (bind _output_get (set `self.VDBMatInst` _returnvalue_2))
      (bind _outrownames_2 (`DataTableFunctionLibrary.GetDataTableRowNames` "/Game/Materials/VDBClouds/DT_VdbTextures.DT_VdbTextures"))
      (bind _returnvalue_3 (`|GetDataTableRow` "/Game/Materials/VDBClouds/DT_VdbTextures.DT_VdbTextures" (`KismetArrayLibrary.Array_Random` _outrownames_2))
        (:`then`
          (`MaterialInstanceDynamic.SetSparseVolumeTextureParameterValue` _output_get "None" (break `/Game/Materials/VDBClouds/ST_VdbTexture` _returnvalue_3)))))))